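; Player wizard character Blueprint that handles the HUD, enemy targeting display, ability animations and touch camera control.
; BeginPlay creates the player UI, Tick refreshes the closest-enemy targeting decal, and an event toggles a BP_AI's health/mana widget.
; Events play basic attack and two skill montages, while touch drags apply yaw from the movement delta.
; ShowDeathScreen and gamepad right-stick events are empty, with leftover game-over, aiming and pitch logic disconnected.
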(event `InputVectorAxis|Gamepad_Right2D`
  (params (AxisValue :type "Vector Structure"))
  ;[0.2135 0.2135 0.2135] TODO
)

(event `self.ReceiveBeginPlay`
  ;[1 0.4279 0.9703] Show Player UI
  (bind _returnvalue (`|CreateWidget` "/Game/BattleWizardPolyart/UI/Widgets/WBP_PlayerUI.WBP_PlayerUI_C"))
  (bind _output_get (set `self.HUD` _returnvalue))
  (`UserWidget.AddToViewport` _output_get 0))

(event `self.ShowHealthManaWidget`
  (params (TargetActor :type "FourCharacter Object Reference") (bValue :type Boolean))
  ;[1 0 0.1986] Show Health and Mana Widget
  (bind _asbp_ai (cast `/Game/BattleWizardPolyart/AI/BP_AI` TargetActor))
  (if bValue
    (bind _healthmanawidget (`FourCharacter.HealthManaWidget` _asbp_ai))
    (`SceneComponent.SetVisibility` _healthmanawidget true false)
    (else
      (`SceneComponent.SetVisibility` _healthmanawidget false false))))

(event `self.ReceiveTick`
  (params (DeltaSeconds :type "Float (single-precision)"))
  ;[0.3926 0.4024 1] Show Closest enemy in range
  (`self.SpawnTargettingDecalOnEnemy`))

(event `self.PlayAttackAnimation`
  ;[1 0.8632 0] Basic Attack Animation
  (bind _returnvalue (`self.PlayAnimMontage` "/Game/BattleWizardPolyart/Animations/AM_BasicAttack.AM_BasicAttack"))
  (`KismetSystemLibrary.Delay` _returnvalue))

(event `self.PlaySkillOneAnimation`
  ;[0.1448 1 0.5143] Skill One Animation
  (bind _returnvalue (`self.PlayAnimMontage` "/Game/BattleWizardPolyart/Animations/AM_Skill1.AM_Skill1"))
  (`KismetSystemLibrary.Delay` (* 2 _returnvalue)))

(event `self.PlaySkillTwoAnimation`
  ;[0 0.8381 1] Skill Two Animation
  (bind _returnvalue (`self.PlayAnimMontage` "/Game/BattleWizardPolyart/Animations/AM_Skill2.AM_Skill2"))
  (`KismetSystemLibrary.Delay` (* 2 _returnvalue))
  (`self.StopAnimMontage` "/Game/BattleWizardPolyart/Animations/AM_Skill2.AM_Skill2"))

(event `self.ShowDeathScreen`
  ;[1 0.391 0.1073] Show End Screen (Doing this in Game Mode)
)

(event `InputTouch`
  (params (Location :type "Vector Structure") (FingerIndex :type "ETouchIndex Enum"))
  ;[1 1 1] Rotate Camera with Touch
  (:`Pressed`
    (set `self.StartLoc` (`KismetMathLibrary.MakeVector2D` Location_X Location_Y) :!label _label))
  (:`Released`
    (goto _label))
  (:`Moved`
    (`self.RotateCam` (`KismetMathLibrary.MakeVector2D` Location_X Location_Y))
    (goto _label)))

(event `RotateCam`
  (params (UpdateLoc :type "Vector2D Structure"))
  (bind (_returnvalue_x _returnvalue_y) (`KismetMathLibrary.BreakVector2D` (- UpdateLoc (`self.StartLoc`))))
  ;[1 1 1] Rotate Camera with Touch
  (`self.AddControllerYawInput` (/ _returnvalue_x 5.0)))

(fn `UserConstructionScript`)