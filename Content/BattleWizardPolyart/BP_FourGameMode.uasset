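; Game mode for a wave-based game that spawns AI enemies and objectives and handles game over.
; StartGame caches spawn locations through EQS queries.
; Spawn events add one random-point enemy per wave and fill a free objective slot, tracked by an occupancy map, clearing their timers at wave 31.
; GameOver shows win/loss and saves through a newly created save object, comparing Score against its default highscore; save-loading logic is unconnected.
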(event `self.GameOver`
  (params (bWonGame :type Boolean))
  (bind _score (`self.Score`))
  ;[0.9366 1 0] Show GameOver Stat
  (bind _returnvalue (`GameplayStatics.CreateSaveGameObject` "/Game/BattleWizardPolyart/BP_FourSaveGame.BP_FourSaveGame_C"))
  (bind _output_get (set `self.SaveGameInstance` _returnvalue))
  (if (> _score (`FourSaveGame.Highscore` _returnvalue))
    (set `FourSaveGame.Highscore` _score _output_get))
  (`AsyncActionHandleSaveGame.AsyncSaveGameToSlot` _returnvalue (`FourSaveGame.SaveSlotName` _returnvalue) (`FourSaveGame.UserIndex` _returnvalue)
    (:`then`
      (if (not bWonGame)
        (`WidgetLayoutLibrary.RemoveAllWidgets`))
      (bind _returnvalue_2 (`|CreateWidget` "/Game/BattleWizardPolyart/UI/Widgets/WBP_GameOver.WBP_GameOver_C"))
      (`UserWidget.AddToViewport` _returnvalue_2 0)
      (`TextBlock.SetText` (`/Game/BattleWizardPolyart/UI/Widgets/WBP_GameOver.GameOver` _returnvalue_2) (select `bool` bWonGame :`false` "YOU LOST!" :`true` "YOU WON!!!" :!type "Text")))))

(event `self.StartGame`
  ;[0.3858 0.05122 1] Get All AISpawnPoints
  (bind _returnvalue (`EnvQueryManager.RunEQSQuery` "/Game/BattleWizardPolyart/AI/EQS_FindSpawnPoint.EQS_FindSpawnPoint" self "AllMatching"))
  (add `EnvQueryInstanceBlueprintWrapper.OnQueryFinishedEvent` _returnvalue (delegate `OnQueryFinishedEvent1`))
  ;[0 0.5432 1] Get All ObjectiveSpawnLocations
  (bind _returnvalue_2 (`EnvQueryManager.RunEQSQuery` "/Game/BattleWizardPolyart/AI/EQS_FindObjSpawnPoint.EQS_FindObjSpawnPoint" self "AllMatching"))
  (add `EnvQueryInstanceBlueprintWrapper.OnQueryFinishedEvent` _returnvalue_2 (delegate `OnQueryFinishedEvent2`)))

(event `OnQueryFinishedEvent1`
  (params (QueryInstance :type "EnvQueryInstanceBlueprintWrapper Object Reference") (QueryStatus :type "EEnvQueryStatus Enum" :default "Processing"))
  ;[0.3858 0.05122 1] Get All AISpawnPoints
  (switch `EEnvQueryStatus` QueryStatus
    (:`Success`
      (bind _resultlocations (`EnvQueryInstanceBlueprintWrapper.GetQueryResultsAsLocations` QueryInstance))
      (set `self.AISpawnLocations` _resultlocations))))

(event `OnQueryFinishedEvent2`
  (params (QueryInstance :type "EnvQueryInstanceBlueprintWrapper Object Reference") (QueryStatus :type "EEnvQueryStatus Enum" :default "Processing"))
  ;[0 0.5432 1] Get All ObjectiveSpawnLocations
  (switch `EEnvQueryStatus` QueryStatus
    (:`Success`
      (bind _resultlocations (`EnvQueryInstanceBlueprintWrapper.GetQueryResultsAsLocations` QueryInstance))
      (for (_array_element _array_index) _resultlocations
        (`BlueprintMapLibrary.Map_Add` (`self.ObjectiveSpawnLocations`) _array_index _array_element)
        ;;[0.02623 0 1] ObjectiveSpawnPoints are Initially Empty (i.e. bool value false)
        (`BlueprintMapLibrary.Map_Add` (`self.Objectives`) _array_index)))))

(event `self.SpawnAIEnemy`
  (bind _aispawnlocations (`self.AISpawnLocations`))
  ;[1 0 0.05924] Spawn AI
  (if (== (`self.WaveNum`) 31)
    (`KismetSystemLibrary.K2_ClearAndInvalidateTimerHandle` (`self.SpawnAITimer`))
    (else
      (bind _asbp_four_character (cast `/Game/BattleWizardPolyart/Player/BP_FourCharacter` (`GameplayStatics.GetPlayerPawn` 0)))
      (`/Game/BattleWizardPolyart/UI/Widgets/WBP_PlayerUI.ShowNotification` (`/Game/BattleWizardPolyart/Player/BP_FourCharacter.HUD` _asbp_four_character) (`|FormatText` "Wave : {Num}" (`self.WaveNum`)))
      (`AIBlueprintHelperLibrary.SpawnAIFromClass` "/Game/BattleWizardPolyart/AI/BP_AI.BP_AI_C" "/Game/BattleWizardPolyart/AI/BT_AI.BT_AI" (`|GetArrayItem` _aispawnlocations (`KismetMathLibrary.RandomIntegerInRange` 0 (- (`KismetArrayLibrary.Array_Length` _aispawnlocations) 1))) (struct) false null)
      (`/Engine/EditorBlueprintResources/StandardMacros.IncrementInt` (`self.WaveNum`)))))

(event `self.SpawnObjective`
  (bind _objectives (`self.Objectives`))
  (bind _objectivespawnlocations (`self.ObjectiveSpawnLocations`))
  ;[0.7346 0.589 1] Spawn Objective only if there are empty Objective Spawn Points
  (if (== (`self.WaveNum`) 31)
    (`KismetSystemLibrary.K2_ClearAndInvalidateTimerHandle` (`self.SpawnObjectiveTimer`))
    (elif (> (`BlueprintMapLibrary.Map_Length` _objectivespawnlocations) 0)
      (bind _keys (`BlueprintMapLibrary.Map_Keys` _objectivespawnlocations))
      (set `self.StopLooping` false)
      (`BlueprintMapLibrary.Map_Keys` _objectives)
      (for _array_element _keys
        (if (not (`self.StopLooping`))
          (bind (_value _returnvalue) (`BlueprintMapLibrary.Map_Find` _objectives _array_element))
          (if _returnvalue
            (if (not _value)
              (`BlueprintMapLibrary.Map_Add` (`self.Objectives`) _array_element true)
              (bind (_value_2 _returnvalue_2) (`BlueprintMapLibrary.Map_Find` (`self.ObjectiveSpawnLocations`) _array_element))
              (if _returnvalue_2
                (`|SpawnActorFromClass` "/Game/BattleWizardPolyart/BP_FourObjectiveActor.BP_FourObjectiveActor_C" (`KismetMathLibrary.MakeTransform` _value_2) "Undefined" "OverrideRootScale" null null)
                (set `self.StopLooping` true)))))))))

(event `self.RemoveObjectiveFromObjectivesArray`
  (params (ObjSpawnLoc :type "Vector Structure"))
  ;[1 1 1] Remove Objective from Array on Destroyed
  (bind _values (`BlueprintMapLibrary.Map_Values` (`self.ObjectiveSpawnLocations`)))
  (if (`KismetArrayLibrary.Array_Contains` _values ObjSpawnLoc)
    (`BlueprintMapLibrary.Map_Add` (`self.Objectives`) (`KismetArrayLibrary.Array_Find` _values ObjSpawnLoc))))

(fn `UserConstructionScript`)