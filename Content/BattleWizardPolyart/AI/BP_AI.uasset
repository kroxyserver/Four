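; AI-controlled character Blueprint with health and mana components, an overhead-style status widget and attack animations.
; BeginPlay caches the widget and sets its maximums from component defaults, then Tick copies current values into it.
; Events play basic attack and two skill montages with length-based delays, and a function sets walk speed.
; AI controller idle-state and spawn-transform logic is present but disconnected, so it never runs.
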(event `self.ReceiveBeginPlay`
  ;[1 1 1] Get a Ref to HealthAndMana AI Widget and Set MaxHealth and MaxMana
  (bind _aswbp_health_and_mana_ai (cast `/Game/BattleWizardPolyart/UI/Widgets/WBP_HealthAndManaAI` (`WidgetComponent.GetUserWidgetObject` (`self.HealthManaWidget`))))
  (bind _output_get (set `self.As WBP Health And Mana AI` _aswbp_health_and_mana_ai))
  (set `/Game/BattleWizardPolyart/UI/Widgets/WBP_HealthAndManaAI.MaxHealth` (`FourHealthComponent.DefaultHealth` (`self.HealthComp`)) _output_get)
  (set `/Game/BattleWizardPolyart/UI/Widgets/WBP_HealthAndManaAI.MaxMana` (`FourManaComponent.DefaultMana` (`self.ManaComp`)) _output_get))

(event `self.ReceiveTick`
  (params (DeltaSeconds :type "Float (single-precision)"))
  (bind _as_wbp_health_and_mana_ai (`self.As WBP Health And Mana AI`))
  ;[1 1 1] Update Health and Mana every Tick
  (set `/Game/BattleWizardPolyart/UI/Widgets/WBP_HealthAndManaAI.CurrentHealth` (`FourHealthComponent.Health` (`self.HealthComp`)) _as_wbp_health_and_mana_ai)
  (set `/Game/BattleWizardPolyart/UI/Widgets/WBP_HealthAndManaAI.CurrentMana` (`FourManaComponent.Mana` (`self.ManaComp`)) _as_wbp_health_and_mana_ai))

(event `self.PlayAttackAnimation`
  ;[1 1 1] Basic Attack Animation
  (bind _returnvalue (`self.PlayAnimMontage` "/Game/BattleWizardPolyart/Animations/AM_BasicAttack.AM_BasicAttack"))
  (`KismetSystemLibrary.Delay` _returnvalue))

(event `self.PlaySkillOneAnimation`
  ;[1 1 1] Skill One Animation
  (bind _returnvalue (`self.PlayAnimMontage` "/Game/BattleWizardPolyart/Animations/AM_Skill1.AM_Skill1"))
  (`KismetSystemLibrary.Delay` (* 2 _returnvalue)))

(event `self.PlaySkillTwoAnimation`
  ;[1 1 1] Skill Two Animation
  (bind _returnvalue (`self.PlayAnimMontage` "/Game/BattleWizardPolyart/Animations/AM_Skill2.AM_Skill2"))
  (`KismetSystemLibrary.Delay` (* 2 _returnvalue))
  (`self.StopAnimMontage` "/Game/BattleWizardPolyart/Animations/AM_Skill2.AM_Skill2"))

(fn `UpdateWalkSpeed`
  (params (NewWalkSpeed :type "Float (double-precision)"))
  (set `CharacterMovementComponent.MaxWalkSpeed` NewWalkSpeed (`self.CharacterMovement`)))

(fn `UserConstructionScript`)